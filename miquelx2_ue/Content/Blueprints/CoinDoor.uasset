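; CoinDoor is a child Blueprint of a door that only responds to a player who holds enough coins.
; On overlap it casts the other actor to MyCharacter and runs the parent overlap logic only if Coins meets or exceeds RequiredCoins, without deducting any.
; End overlap always passes straight to the parent, which holds the actual door behavior.
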(event `self.ReceiveActorBeginOverlap`
  (params (OtherActor :type "Actor Object Reference"))
  (bind _asmy_character (cast `/Game/Blueprints/MyCharacter` OtherActor))
  (if (>= (`/Game/Blueprints/MyCharacter.Coins` _asmy_character) (`self.requiredCoins`))
    (`parent.ReceiveActorBeginOverlap` _asmy_character)))

(event `self.ReceiveActorEndOverlap`
  (params (OtherActor :type "Actor Object Reference"))
  (`parent.ReceiveActorEndOverlap` OtherActor))

(fn `UserConstructionScript`
  (`parent.UserConstructionScript`))